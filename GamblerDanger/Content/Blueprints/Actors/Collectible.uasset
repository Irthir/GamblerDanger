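; Collectible pickup actor that adds one point to the player's score.
; Its Carte component spins around yaw on Tick, with an overlap handler bound on BeginPlay.
; The handler matches the overlapping actor by display name "BP_Joueur", increments Score on the InterfaceJoueur of the BP_Joueur found via GetActorOfClass, then destroys itself.
; A cast-based version of the score increment remains unconnected.
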(event Custom|OverlapPlayer
  (params (OverlappedComponent :type Primitive%20Component%20Object%20Reference) (OtherActor :type Actor%20Object%20Reference) (OtherComp :type Primitive%20Component%20Object%20Reference) (OtherBodyIndex :type Integer) (bFromSweep :type Boolean) (SweepResult :type Hit%20Result%20Structure%20%28by%20ref%29))
  (if (Utilities|Enum|Equal(Enum) (Utilities|GetDisplayName OtherActor) "BP_Joueur")
    (bind _returnvalue (Actor|GetActorOfClass "/Game/Blueprints/Pawns/BP_Joueur.BP_Joueur_C"))
    (Math|Integer|IncrementInt (Variables|/Game/Blueprints/Widget/InterfaceJoueur.InterfaceJoueur_C|GetScore (Variables|/Game/Blueprints/Pawns/BP_Joueur.BP_Joueur_C|GetInterfaceJoueur _returnvalue))
      (:%20%20
        (Actor|DestroyActor self)))))

(event EventBeginPlay
  (Collision|AssignOnComponentBeginOverlap (Variables|Default|GetCarte) (delegate Custom|OverlapPlayer)))

(event Collision|EventActorBeginOverlap
  (params (OtherActor :type Actor%20Object%20Reference)))

(event EventTick
  (params (DeltaSeconds :type Float%20%28single-precision%29))
  (Transformation|AddRelativeRotation (Variables|Default|GetCarte) (Math|Rotator|MakeRotator 0.0 0.0 (* DeltaSeconds 1.8e+02)) false false))

(fn ConstructionScript)