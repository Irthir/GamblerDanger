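; CameraJoueur is a camera actor that follows the player's BP_Joueur character.
; Each Tick it finds and caches the first BP_Joueur if none is valid, otherwise updates position and rotation.
; It teleports to the player's X, offset back along Y by DistanceJoueur at a fixed height.
; It then uses a look-at rotation toward the player at that same height, keeping the view level.
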(event Custom|PositionCamera
  (bind _joueur (Variables|Default|GetJoueur))
  (bind _returnvalue (Transformation|GetActorLocation _joueur))
  (Transformation|SetActorLocation (Math|Vector|MakeVector (.x _returnvalue) (- (.y _returnvalue) (Variables|Default|GetDistanceJoueur)) 2e+02) false true))

(event Custom|RotationCamera
  (bind _joueur (Variables|Default|GetJoueur))
  (bind _returnvalue (Transformation|GetActorLocation _joueur))
  (Transformation|SetActorRotation (Math|Rotator|FindLookatRotation (Transformation|GetActorLocation) (Math|Vector|MakeVector (.x _returnvalue) (.y _returnvalue) 2e+02)) true))

(event Custom|SetJoueur
  (bind _returnvalue (Actor|GetActorOfClass "/Game/Blueprints/Pawns/BP_Joueur.BP_Joueur_C"))
  (Variables|Default|SetJoueur _returnvalue))

(event EventBeginPlay)

(event Collision|EventActorBeginOverlap
  (params (OtherActor :type Actor%20Object%20Reference)))

(event EventTick
  (params (DeltaSeconds :type Float%20%28single-precision%29))
  (Utilities|IsValid (Variables|Default|GetJoueur)
    (:Is%20Valid
      (CallFunction|PositionCamera)
      (CallFunction|RotationCamera))
    (:Is%20Not%20Valid
      (CallFunction|SetJoueur))))

(fn ConstructionScript)