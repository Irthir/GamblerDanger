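; Pique is a spike hazard actor that damages the player when touched.
; On BeginPlay it binds the begin-overlap events of its five cone components to a single OverlapPlayer handler.
; The handler checks that the other actor's display name equals "BP_Joueur", casts it to that class and calls its Degats function.
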(event Custom|OverlapPlayer
  (params (OverlappedComponent :type Primitive%20Component%20Object%20Reference) (OtherActor :type Actor%20Object%20Reference) (OtherComp :type Primitive%20Component%20Object%20Reference) (OtherBodyIndex :type Integer) (bFromSweep :type Boolean) (SweepResult :type Hit%20Result%20Structure%20%28by%20ref%29))
  (if (Utilities|Enum|Equal(Enum) (Utilities|GetDisplayName OtherActor) "BP_Joueur")
    (bind _asbp_joueur (Utilities|Casting|CastToBP_Joueur OtherActor))
    (Default|Degats _asbp_joueur)))

(event EventBeginPlay
  (Collision|AssignOnComponentBeginOverlap (Variables|Default|GetCone2) (delegate Custom|OverlapPlayer)))

(event Collision|EventActorBeginOverlap
  (params (OtherActor :type Actor%20Object%20Reference)))

(event EventTick
  (params (DeltaSeconds :type Float%20%28single-precision%29)))

(fn ConstructionScript)