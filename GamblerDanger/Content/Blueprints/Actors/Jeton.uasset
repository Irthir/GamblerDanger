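; Jeton is a reusable projectile actor tied to a Distributeur, damaging the player or destroying Destructible actors on contact.
; While Feu is set, Tick moves it along Direction at FVitesse with sweep.
; Cylinder overlaps ignore Distributeur, spawn-point volumes and Collectibles.
; Any other overlap teleports it back to its BeginPlay origin, stops it and calls Recharge on the Distributeur, with overlap events briefly disabled during the reset.
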(event OnComponentBeginOverlap(Cylinder)
  (params (OverlappedComponent :type Primitive%20Component%20Object%20Reference) (OtherActor :type Actor%20Object%20Reference) (OtherComp :type Primitive%20Component%20Object%20Reference) (OtherBodyIndex :type Integer) (bFromSweep :type Boolean) (SweepResult :type Hit%20Result%20Structure%20%28by%20ref%29))
  (Utilities|Casting|CastToDistributeur OtherActor
    (:CastFailed
      (Utilities|Casting|CastToTriggerVolumeSpawnPoint OtherActor
        (:CastFailed
          (Utilities|Casting|CastToCollectible OtherActor
            (:CastFailed
              (Variables|/Script/Engine.PrimitiveComponent|SetbGenerateOverlapEvents (Variables|Default|GetCylinder) false)
              (CallFunction|Reset)
              (Variables|/Script/Engine.PrimitiveComponent|SetbGenerateOverlapEvents (Variables|Default|GetCylinder) true)
              (bind _asbp_joueur (Utilities|Casting|CastToBP_Joueur OtherActor)
                (:then
                  (Default|Degats _asbp_joueur))
                (:CastFailed
                  (bind _asdestructible (Utilities|Casting|CastToDestructible OtherActor)
                    (:then
                      (Default|Detruire _asdestructible))
                    (:CastFailed
                      (if (Variables|Default|GetbDebug)
                        (Development|PrintString (Utilities|GetDisplayName OtherActor))))))))))))))

(event Custom|Reset
  (Transformation|SetActorLocation (Variables|Default|GetOrigine) false true)
  (Variables|Default|SetbFeu false)
  (Default|Recharge (Variables|Default|GetDistributeur)))

(event EventBeginPlay
  (Variables|Default|SetOrigine (Transformation|GetActorLocation)))

(event Collision|EventActorBeginOverlap
  (params (OtherActor :type Actor%20Object%20Reference)))

(event EventTick
  (params (DeltaSeconds :type Float%20%28single-precision%29))
  (if (Variables|Default|GetbFeu)
    (Transformation|SetActorLocation (+ (Transformation|GetActorLocation) (* (Variables|Default|GetDirection) (* DeltaSeconds (Variables|Default|GetfVitesse)))) true false)))

(fn ConstructionScript)