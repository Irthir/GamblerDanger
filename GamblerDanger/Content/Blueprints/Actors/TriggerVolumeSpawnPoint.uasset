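; Trigger volume actor that sets the respawn value on the player when touched, apparently serving as a spawn checkpoint.
; On BeginPlay it binds the Cube component's begin-overlap event.
; An overlapping actor whose display name equals "BP_Joueur" is cast to BP_Joueur and receives this volume's NRespawn.
; Debug prints show a greeting for the player or the name of any other overlapping actor.
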(event Custom|OverlapPlayer
  (params (OverlappedComponent :type Primitive%20Component%20Object%20Reference) (OtherActor :type Actor%20Object%20Reference) (OtherComp :type Primitive%20Component%20Object%20Reference) (OtherBodyIndex :type Integer) (bFromSweep :type Boolean) (SweepResult :type Hit%20Result%20Structure%20%28by%20ref%29))
  (bind _returnvalue (Utilities|GetDisplayName OtherActor))
  (if (Utilities|Enum|Equal(Enum) _returnvalue "BP_Joueur")
    (bind _asbp_joueur (Utilities|Casting|CastToBP_Joueur OtherActor))
    (Variables|/Game/Blueprints/Pawns/BP_Joueur.BP_Joueur_C|SetnRespawn _asbp_joueur (Variables|Default|GetnRespawn))
    (Development|PrintString "Hello")
    (else
      (Development|PrintString _returnvalue))))

(event EventBeginPlay
  (Collision|AssignOnComponentBeginOverlap (Variables|Default|GetCube) (delegate Custom|OverlapPlayer)))

(fn ConstructionScript)