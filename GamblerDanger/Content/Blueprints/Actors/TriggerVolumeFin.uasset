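; End-of-game trigger volume that fires when the player walks into its Cube.
; On BeginPlay it binds the Cube's begin-overlap event, casts the overlapping actor to BP_Joueur, sets the Fin flag on that player's InterfaceJoueur and shows the mouse cursor.
; An older display-name check for BP_Joueur is left in the graph but never runs.
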(event Custom|OverlapPlayer
  (params (OverlappedComponent :type Primitive%20Component%20Object%20Reference) (OtherActor :type Actor%20Object%20Reference) (OtherComp :type Primitive%20Component%20Object%20Reference) (OtherBodyIndex :type Integer) (bFromSweep :type Boolean) (SweepResult :type Hit%20Result%20Structure%20%28by%20ref%29))
  (bind _asbp_joueur (Utilities|Casting|CastToBP_Joueur OtherActor))
  (Variables|/Game/Blueprints/Widget/InterfaceJoueur.InterfaceJoueur_C|SetbFin (Variables|/Game/Blueprints/Pawns/BP_Joueur.BP_Joueur_C|GetInterfaceJoueur _asbp_joueur) true)
  (Variables|/Script/Engine.PlayerController|SetbShowMouseCursor (Game|GetPlayerController 0) true))

(event EventBeginPlay
  (Collision|AssignOnComponentBeginOverlap (Variables|Default|GetCube) (delegate Custom|OverlapPlayer)))

(fn ConstructionScript)