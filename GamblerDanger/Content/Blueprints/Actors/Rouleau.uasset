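; Rouleau is an interactive roller actor with three parts that the player cycles through three arrangements by pressing Tab while inside its Volume.
; Volume overlaps set a presence flag by matching the other actor's display name to BP_Joueur, and input is enabled on BeginPlay.
; Each press advances Etat modulo three, prints it, and calls TourneRouleau, which fakes rotation by teleporting the parts to preset vertical offsets.
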(event OnComponentBeginOverlap(Volume)
  (params (OverlappedComponent :type Primitive%20Component%20Object%20Reference) (OtherActor :type Actor%20Object%20Reference) (OtherComp :type Primitive%20Component%20Object%20Reference) (OtherBodyIndex :type Integer) (bFromSweep :type Boolean) (SweepResult :type Hit%20Result%20Structure%20%28by%20ref%29))
  (if (Utilities|Enum|Equal(Enum) (Utilities|GetDisplayName OtherActor) "BP_Joueur")
    (Variables|Default|SetJoueurPresent true)))

(event OnComponentEndOverlap(Volume)
  (params (OverlappedComponent :type Primitive%20Component%20Object%20Reference) (OtherActor :type Actor%20Object%20Reference) (OtherComp :type Primitive%20Component%20Object%20Reference) (OtherBodyIndex :type Integer))
  (if (Utilities|Enum|Equal(Enum) (Utilities|GetDisplayName OtherActor) "BP_Joueur")
    (Variables|Default|SetJoueurPresent false)))

(event Custom|ChangementEtat
  (Math|Integer|IncrementInt (Variables|Default|GetEtat)
    (:%20%20
      (Variables|Default|SetEtat (Math|Integer|%(Integer) (Variables|Default|GetEtat) 3))
      (Development|PrintString (Utilities|String|ToString(Integer) (Variables|Default|GetEtat)))
      (CallFunction|TourneRouleau))))

(event Custom|TourneRouleau
  (switch int (Variables|Default|GetEtat)
    (:Default
      (Transformation|SetRelativeLocation (Variables|Default|GetPartieRouleau1) "0, 0, 0" false true :!label _label)
      (Transformation|SetRelativeLocation (Variables|Default|GetPartieRouleau2) "0, 0, 0" false true)
      (Transformation|SetRelativeLocation (Variables|Default|GetPartieRouleau3) "0, 0, 0" false true))
    (:0
      (goto _label))
    (:1
      (Transformation|SetRelativeLocation (Variables|Default|GetPartieRouleau1) "0,0.000000,1000.000000" false true)
      (Transformation|SetRelativeLocation (Variables|Default|GetPartieRouleau2) "0, 0,-500.000000" false true)
      (Transformation|SetRelativeLocation (Variables|Default|GetPartieRouleau3) "0, 0,-500.000000" false true))
    (:2
      (Transformation|SetRelativeLocation (Variables|Default|GetPartieRouleau1) "0, 0,500.000000" false true)
      (Transformation|SetRelativeLocation (Variables|Default|GetPartieRouleau2) "0, 0,500.000000" false true)
      (Transformation|SetRelativeLocation (Variables|Default|GetPartieRouleau3) "0, 0,1000.000000" false true))))

(event EventBeginPlay
  (Input|EnableInput (Game|GetPlayerController 0)))

(event Collision|EventActorBeginOverlap
  (params (OtherActor :type Actor%20Object%20Reference)))

(event EventTick
  (params (DeltaSeconds :type Float%20%28single-precision%29)))

(event Input|KeyboardEvents|Tab
  (params (Key :type Key%20Structure :default "None"))
  (:Pressed
    (if (Variables|Default|GetJoueurPresent)
      (CallFunction|ChangementEtat))))

(fn ConstructionScript)