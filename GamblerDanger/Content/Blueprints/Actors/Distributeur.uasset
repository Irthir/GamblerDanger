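; Distributeur is a dispenser actor that spawns and controls a single Jeton (token) through a timed recharge-and-fire cycle.
; On BeginPlay it spawns the Jeton offset along world X, then gives it a back-reference and that origin point.
; Recharge arms a Tick-accumulated timer that, once it reaches FAttente, calls Feu to disarm itself and set the Feu flag on the same Jeton.
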(event Custom|Recharge
  (Variables|Default|SetbFeu true))

(event Custom|Feu
  (Variables|Default|SetbFeu false)
  (Variables|Default|SetfTemps 0.0)
  (Variables|/Game/Blueprints/Actors/Jeton.Jeton_C|SetbFeu (Variables|Default|GetJeton) true))

(event EventBeginPlay
  (bind _returnvalue (Transformation|GetActorTransform))
  (bind _returnvalue_2 (Math|Vector|MakeVector -1e+02 0.0 0.0))
  (bind _returnvalue_3 (+ (.location _returnvalue) _returnvalue_2))
  (bind _returnvalue_4 (Game|SpawnActorfromClass "/Game/Blueprints/Actors/Jeton.Jeton_C" (Math|Transform|MakeTransform _returnvalue_3 (.rotation _returnvalue) (.scale _returnvalue)) "AlwaysSpawn" 0 0))
  (bind _output_get (Variables|Default|SetJeton _returnvalue_4))
  (Variables|/Game/Blueprints/Actors/Jeton.Jeton_C|SetDistributeur _output_get self)
  (Variables|/Game/Blueprints/Actors/Jeton.Jeton_C|SetOrigine _output_get _returnvalue_3))

(event Collision|EventActorBeginOverlap
  (params (OtherActor :type Actor%20Object%20Reference)))

(event EventTick
  (params (DeltaSeconds :type Float%20%28single-precision%29))
  (if (Variables|Default|GetbFeu)
    (Variables|Default|SetfTemps (+ (Variables|Default|GetfTemps) DeltaSeconds))
    (if (>= (Variables|Default|GetfTemps) (Variables|Default|GetfAttente))
      (CallFunction|Feu))))

(fn ConstructionScript)